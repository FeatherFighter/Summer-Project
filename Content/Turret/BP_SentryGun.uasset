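; BP_SentryGun is a sentry turret actor that turns toward pawns it sees and fires at them.
; PawnSensing's OnSeePawn event snaps the actor's rotation to face the seen pawn, with no filtering by pawn type.
; After a short Delay, it spawns BP_SentryGunAmmo at the PointingDirection component's world transform.
; A laser gunshot sound node exists but is disconnected, so it never plays.
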(event OnSeePawn(PawnSensing)
  (params (Pawn :type Pawn%20Object%20Reference))
  (Transformation|SetActorRotation (Math|Rotator|FindLookatRotation (Transformation|GetActorLocation) (Transformation|GetActorLocation Pawn)))
  (Utilities|FlowControl|Delay 0.2)
  (Game|SpawnActorfromClass "/Game/Turret/BP_SentryGunAmmo.BP_SentryGunAmmo_C" (Transformation|GetWorldTransform (Variables|Default|GetPointingDirection)) "Undefined" "MultiplyWithRoot" 0 0))

(fn ConstructionScript)