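; Actor component that makes the first light component found on its owner pulse smoothly between minimum and maximum intensity.
; BeginPlay caches that light and sets it to minimum intensity.
; Tick wraps accumulated time by PulseRate, which acts as the cycle length in seconds, and feeds the phase through a sine wave.
; The sine is mapped inversely onto the intensity range, so its trough gives the brightest light.
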(event EventBeginPlay
  (bind _output_get (Variables|Default|SetControlLight (Actor|GetComponentbyClass (Components|GetOwner) "/Script/Engine.LightComponent")))
  (Utilities|IsValid _output_get
    (:Is%20Valid
      (Rendering|Components|Light|SetIntensity _output_get (Variables|Default|GetMinLightIntensity)))))

(event EventTick
  (params (DeltaSeconds :type Float%20%28single-precision%29))
  (bind _pulserate (Variables|Default|GetPulseRate))
  (bind _output_get (Variables|Default|SetProgressTime (Math|Float|%(Float) (+ DeltaSeconds (Variables|Default|GetProgressTime)) _pulserate)))
  (bind _output_get_2 (Variables|Default|SetProgressAlpha (/ _output_get _pulserate)))
  (bind _controllight (Variables|Default|GetControlLight)
    (:then
      (Rendering|Components|Light|SetIntensity _controllight (Math|Float|MapRangeClamped (Math|Trig|Sin(Degrees) (* _output_get_2 3.6e+02)) -1.0 1.0 (Variables|Default|GetMaxLightIntensity) (Variables|Default|GetMinLightIntensity))))
    (:else)))