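; BP_SentryGun is an unfinished enemy sentry turret with Searching and Shooting states.
; Tick dispatches on TurretState to a rotation event or an empty Shoot stub, with no state changes here.
; Rotation loops -5 degree yaw steps within a single call while yaw is between 0 and -65.
; Pawn sensing stores the location of pawns tagged Shootable, which nothing uses yet.
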(event OnSeePawn(PawnSensing)
  (params (Pawn :type Pawn%20Object%20Reference))
  (if (Actor|ActorHasTag Pawn "Shootable")
    (Variables|Default|SetNewVar (Transformation|GetActorLocation Pawn))))

(event Custom|Rotate_Turret
  (bind _returnvalue (Transformation|GetActorRotation))
  (while (and (< (.yaw _returnvalue) 0.0) (> (.yaw _returnvalue) -65.0))
    (Transformation|SetActorRotation (Math|Rotator|MakeRotator 0.0 0.0 (+ (.yaw _returnvalue) -5.0)))))

(event Custom|Shoot)

(event EventBeginPlay)

(event Collision|EventActorBeginOverlap
  (params (OtherActor :type Actor%20Object%20Reference)))

(event EventTick
  (params (DeltaSeconds :type Float%20%28single-precision%29))
  (switch Utilities|FlowControl|Switch|SwitchonEnum_SentryGun (Variables|Default|GetTurretState)
    (:NewEnumerator0
      (CallFunction|RotateTurret))
    (:NewEnumerator1
      (CallFunction|Shoot))))

(fn ConstructionScript)